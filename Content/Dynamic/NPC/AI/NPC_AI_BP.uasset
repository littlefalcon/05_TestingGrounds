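; AI controller for guard NPCs that initializes a patrol blackboard and runs the guard behavior tree on BeginPlay.
; Perception updates for actors without the "Enemy" tag set player pawn 0 as the blackboard enemy when sensed, and clear it otherwise.
; Tick mirrors whether a focus actor exists into the controlled AI pawn's Aiming flag.
; An uncalled debug helper prints pawn, sense and object names.
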(event `self.ReceiveBeginPlay`
  (bind _blackboardcomponent (`self.UseBlackboard` "/Game/Dynamic/NPC/AI/PatrolData.PatrolData"))
  (`self.RunBehaviorTree` "/Game/Dynamic/NPC/AI/GuardBehavior.GuardBehavior")
  (set `self.BBComp` _blackboardcomponent))

(event `self.ReceiveTick`
  (params (DeltaSeconds :type "Float (single-precision)"))
  (bind _asai (cast `/Game/Dynamic/NPC/Behavior/AI` (`self.K2_GetPawn`)))
  (set `/Game/Dynamic/NPC/Behavior/AI.Aiming` (`KismetSystemLibrary.IsValid` (`self.GetFocusActor`)) _asai))

(event `self.AIPerception.OnTargetPerceptionUpdated`
  (params (Actor :type "Actor Object Reference") (Stimulus :type "AIStimulus Structure"))
  (bind _enemykey (`self.EnemyKey`))
  (bind _bbcomp (`self.BBComp`))
  (if (`self.ActorHasTag` Actor "Enemy")
    _
    (elif (`.bSuccessfullySensed` (break `AIStimulus` Stimulus))
      (`BlackboardComponent.SetValueAsObject` _bbcomp _enemykey (`GameplayStatics.GetPlayerPawn` 0))
      (else
        (`BlackboardComponent.ClearValue` _bbcomp _enemykey)))))

(fn `Print AI Sense`
  (params (Object :type "Object Object Reference") (Stimulus :type "AIStimulus Structure (by ref)"))
  (bind _returnvalue (`AIPerceptionSystem.GetSenseClassForStimulus` Stimulus))
  (`KismetSystemLibrary.PrintString` (`KismetStringLibrary.Concat_StrStr` (`KismetSystemLibrary.GetObjectName` (`self.K2_GetPawn`)) " " (`KismetSystemLibrary.GetClassDisplayName` _returnvalue) " " (`KismetSystemLibrary.GetObjectName` Object))))

(fn `UserConstructionScript`)